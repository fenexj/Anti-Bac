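; NewPC, apparently a player controller, lets the player push physics objects by holding the left mouse button over them.
; The button opens and closes a Gate on Tick, which traces from the deprojected cursor against PhysicsBody objects with per-frame debug drawing.
; Each hit spawns a small particle effect and, on simulating components, applies a random-strength impulse along the cursor ray at the impact point and bone.
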(event EventBeginPlay)

(event EventTick
  (params (DeltaSeconds :type Float%20%28single-precision%29))
  (bind (_worldlocation _worlddirection _returnvalue) (Game|Player|ConvertMouseLocationToWorldSpace))
  (Utilities|FlowControl|Gate true
    (:Exit
      (if _returnvalue
        (bind (_outhit _returnvalue_2) (Collision|LineTraceForObjects _worldlocation (+ _worldlocation (* _worlddirection 5e+03)) (Utilities|Array|MakeArray "ObjectTypeQuery4") false 0 "ForOneFrame"))
        (if _returnvalue_2
          (Effects|SpawnEmitteratLocation "/Game/FX/NewParticleSystem.NewParticleSystem" (.Location (Collision|BreakHitResult _outhit)) "0, 0, 0" "0.100000,0.100000,0.100000")
          (if (Physics|IsSimulatingPhysics (.HitComponent (Collision|BreakHitResult _outhit)) (.HitBoneName (Collision|BreakHitResult _outhit)))
            (Physics|AddImpulseatLocation (.HitComponent (Collision|BreakHitResult _outhit)) (* _worlddirection (Math|Random|RandomFloatinRange 15.0 45.0)) (.ImpactPoint (Collision|BreakHitResult _outhit)) (.HitBoneName (Collision|BreakHitResult _outhit)))))))))

(event Input|MouseEvents|LeftMouseButton
  (params (Key :type Key%20Structure))
  (bind (_worldlocation _worlddirection _returnvalue) (Game|Player|ConvertMouseLocationToWorldSpace))
  (:Pressed
    (Utilities|FlowControl|Gate true) ; enters at Open
  )
  (:Released
    (Utilities|FlowControl|Gate true) ; enters at Close
  ))

(fn ConstructionScript)